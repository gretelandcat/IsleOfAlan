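; Player character Blueprint for the island game that finds and highlights nearby interactable actors in front of it.
; Each tick it writes its location to a material parameter collection, then sphere-overlaps, filters by InteractionInterface and forward dot product, and highlights the nearest match.
; Interact messages that actor, while AI move requests and the active interaction actor pass to IslandGame_PC.
; Interaction events also set the focused actor, and stopping resets camera state.
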(event `self.ReceiveBeginPlay`
  (`parent.ReceiveBeginPlay`)
  (bind _asisland_game_pc (cast `/Game/Game/IslandGame_PC` (`self.GetController`)))
  (set `self.IslandPlayerController` _asisland_game_pc))

(event `self.ReceiveTick`
  (params (DeltaSeconds :type "Float (single-precision)"))
  (bind _currentfacingactor (`self.CurrentFacingActor`))
  (`parent.ReceiveTick` DeltaSeconds)
  (`KismetMaterialLibrary.SetVectorParameterValue` "/Game/catstuff/Asset_Chunks/foli2/Flowers/MyPlayerPosition.MyPlayerPosition" "PlayerPosition" (`KismetMathLibrary.Conv_VectorToLinearColor` (`self.K2_GetActorLocation`)))
  (bind _facingactor (`self.CheckForFacingActor` null))
  (`/Engine/EditorBlueprintResources/StandardMacros.IsValid` _facingactor
    (:`Is Valid`
      (`/Engine/EditorBlueprintResources/StandardMacros.IsValid` _currentfacingactor
        (:`Is Valid`
          (message `/Game/Game/InteractionInterface.DeHighlight` _currentfacingactor))
        (:`Is Not Valid`
          _))
      (message `/Game/Game/InteractionInterface.Highlight` _facingactor)
      (set `self.CurrentFacingActor` _facingactor))
    (:`Is Not Valid`
      (`/Engine/EditorBlueprintResources/StandardMacros.IsValid` _currentfacingactor
        (:`Is Valid`
          (message `/Game/Game/InteractionInterface.DeHighlight` _currentfacingactor)
          (set `self.CurrentFacingActor` null))))))

(event `self.Interact`
  (params (InstigatingCharacter :type "/Game/Characters/IslandCharacter_C Object Reference") (`AI Interact Task` :type "/Game/Characters/NPC/AI/Tasks/Interact_Task Object Reference"))
  (message `/Game/Game/InteractionInterface.Interact` (`self.CurrentFacingActor`) self null))

(event `PlayerAIMoveTo`
  (params (TargetLocation :type "Vector Structure") (MoveInstigatingActor :type "Actor Object Reference"))
  (`/Game/Game/IslandGame_PC.StartPlayerAIMoveTo` (`self.IslandPlayerController`) TargetLocation MoveInstigatingActor))

(event `self.SetInteraction`
  (params (InteractionActor :type "Actor Object Reference") (FocalActor :type "Actor Object Reference"))
  (bind _asisland_game_pc (cast `/Game/Game/IslandGame_PC` (`self.GetController`)))
  (set `/Game/Game/IslandGame_PC.CurrentInteractionActor` InteractionActor _asisland_game_pc)
  (set `self.CurrentFocusedActor` (select `bool` (`KismetSystemLibrary.IsValid` FocalActor) :`false` self :`true` FocalActor :!type "Actor Object Reference")))

(event `self.StopInteraction`
  (bind _asisland_game_pc (cast `/Game/Game/IslandGame_PC` (`self.GetController`)))
  (set `/Game/Game/IslandGame_PC.CurrentInteractionActor` null _asisland_game_pc)
  (set `self.CurrentFocusedActor` null)
  (set `self.CurrentCameraState` "NewEnumerator0"))

(fn `CheckForFacingActor`
  (params (ActorClassFilter :type "Object Class Reference"))
  (returns (FacingActor :type "Actor Object Reference"))
  (bind (_outactors _returnvalue) (`KismetSystemLibrary.SphereOverlapActors` (`self.K2_GetActorLocation`) 250.0 (`|MakeArray` "ObjectTypeQuery3" "ObjectTypeQuery1" "ObjectTypeQuery2" "ObjectTypeQuery5" :!type "EObjectTypeQuery Enum")))
  (if _returnvalue
    (bind _returnedactors (`self.FilterActorsByInterface` _outactors "/Game/Game/InteractionInterface.InteractionInterface_C"))
    (bind _actorsbydot (`self.FindFacingActors` _returnedactors 0.5))
    (return (`.ReturnValue` (`GameplayStatics.FindNearestActor` (`self.K2_GetActorLocation`) _actorsbydot)))))

(fn `FilterActorsByInterface`
  (params (IncomingActors :type "Array of Actor Object Reference") (Interface :type "Interface Class Reference"))
  (returns (ReturnedActors :type "Array of Actor Object Reference"))
  (locals (LocalActors :type "Array of Actor Object Reference"))
  (for _array_element IncomingActors
    (if (`KismetSystemLibrary.DoesImplementInterface` _array_element Interface)
      (`KismetArrayLibrary.Array_Add` (`local.LocalActors`) _array_element)))
  (return (`local.LocalActors`)))

(fn `FindFacingActors`
  (params (FoundActors :type "Array of Actor Object Reference") (DotProductCutOff :type "Float (double-precision)"))
  (returns (ActorsByDot :type "Array of Actor Object Reference"))
  (locals (LocalActorsByDot :type "Map of Float (double-precision) to Actor Object Reference") (LocalActors :type "Array of Actor Object Reference"))
  (for _array_element FoundActors
    (bind _returnvalue (`KismetMathLibrary.Dot_VectorVector` (`KismetMathLibrary.Normal` (- (`self.K2_GetActorLocation` _array_element) (`self.K2_GetActorLocation`))) (`self.GetActorForwardVector`)))
    (if (> _returnvalue DotProductCutOff)
      (`BlueprintMapLibrary.Map_Add` (`local.LocalActorsByDot`) _returnvalue _array_element)))
  (bind _keys (`BlueprintMapLibrary.Map_Keys` (`local.LocalActorsByDot`)))
  (`KismetArrayLibrary.SortFloatArray` _keys)
  (for _array_element_2 _keys
    (`KismetArrayLibrary.Array_Add` (`local.LocalActors`) (`BlueprintMapLibrary.Map_Find` (`local.LocalActorsByDot`) _array_element_2)))
  (return (`local.LocalActors`)))

(fn `UserConstructionScript`
  (`parent.UserConstructionScript`))