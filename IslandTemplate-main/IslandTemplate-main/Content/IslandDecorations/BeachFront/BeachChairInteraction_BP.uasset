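; Interactable beach chair Blueprint that lets a player or AI character walk over and play paired character and chair animations.
; Interact moves the character to an Arrow component, trusting the player to report arrival, then snaps it in place with collision off.
; Optional in, action and out montages chain on Blend Out, with the action looping if enabled.
; AI tasks receive completion or failed-move reports, and exiting restores collision and frees the chair.
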(event `self.Highlight`
  (`/Engine/EditorBlueprintResources/StandardMacros.IsValid` (`self.Instigating Character`)
    (:`Is Not Valid`
      (`parent.Highlight`))))

(event `ReplayMontage`
  (bind _charactermontageout (`self.CharacterMontageOut`))
  (bind _instigating_character (`self.Instigating Character`))
  (bind _interacttask (`self.InteractTask`))
  (bind _stationanimationaction (`self.StationAnimationAction`))
  (bind _stationanimationout (`self.StationAnimationOut`))
  (bind _charactermontageout_2 (`self.CharacterMontageOut`))
  (bind _instigating_character_2 (`self.Instigating Character`))
  ; Play Action Animations, report action completed, loop if necessary
  (`|PlayMontage` (`Character.Mesh` (`self.Instigating Character`)) (`self.CharacterMontageAction`) :!label _label
    (:`then`
      (`/Engine/EditorBlueprintResources/StandardMacros.IsValid` _stationanimationaction
        (:`Is Valid`
          (`SkeletalMeshComponent.PlayAnimation` (`self.SkeletalMesh`) _stationanimationaction false))))
    (:`OnBlendOut`
      (`/Engine/EditorBlueprintResources/StandardMacros.IsValid` (`self.Instigating Character`)
        (:`Is Valid`
          (`/Engine/EditorBlueprintResources/StandardMacros.IsValid` _interacttask
            (:`Is Valid`
              (`/Game/Characters/NPC/AI/Tasks/Interact_Task.ReportIneractCompleted` _interacttask))
            (:`Is Not Valid`
              _))
          (if (and (`KismetSystemLibrary.IsValid` _instigating_character) (`self.LoopActivity`) (or (!= (`Character.GetCurrentMontage` _instigating_character) _charactermontageout) (not (`KismetSystemLibrary.IsValid` _charactermontageout))))
            (`self.ReplayMontage`)
            (else
              ; Stop Interacting
              (`/Engine/EditorBlueprintResources/StandardMacros.IsValid` _charactermontageout_2 :!label _label_2
                (:`Is Valid`
                  (`|PlayMontage` (`Character.Mesh` (`self.Instigating Character`)) _charactermontageout_2
                    (:`then`
                      (`/Engine/EditorBlueprintResources/StandardMacros.IsValid` _stationanimationout
                        (:`Is Valid`
                          (`SkeletalMeshComponent.PlayAnimation` (`self.SkeletalMesh`) _stationanimationout false))))
                    (:`OnBlendOut`
                      (`/Game/Game/InteractionInterface.StopInteraction` _instigating_character_2 :!label _label_3)
                      (`self.SetActorEnableCollision` _instigating_character_2 true)
                      (set `self.Instigating Character` null))))
                (:`Is Not Valid`
                  (goto _label_3))))))))))

(event `self.Interact`
  (params (InstigatingCharacter :type "/Game/Characters/IslandCharacter_C Object Reference") (`AI Interact Task` :type "/Game/Characters/NPC/AI/Tasks/Interact_Task Object Reference"))
  (bind _arrow (`self.Arrow`))
  (bind _interacttask (`self.InteractTask`))
  (bind _instigating_character (`self.Instigating Character`))
  (bind _stationanimationin (`self.StationAnimationIn`))
  (bind _charactermontagein (`self.CharacterMontageIn`))
  (bind (_returnvalue_x _returnvalue_y) (`KismetMathLibrary.BreakVector` (`SceneComponent.K2_GetComponentLocation` _arrow)))
  (bind (_returnvalue_x_2 _returnvalue_y_2) (`KismetMathLibrary.BreakVector` (`SceneComponent.K2_GetComponentLocation` (`self.Arrow`))))
  (bind (_returnvalue_x_3 _returnvalue_y_3) (`KismetMathLibrary.BreakVector` (`SceneComponent.K2_GetComponentLocation` (`self.Arrow`))))
  (bind (_returnvalue_x_4 _returnvalue_y_4 _returnvalue_z) (`KismetMathLibrary.BreakVector` (`self.K2_GetActorLocation` _instigating_character)))
  ; Begin Interaction Process
  (`/Engine/EditorBlueprintResources/StandardMacros.IsValid` (`self.Instigating Character`)
    (:`Is Not Valid`
      (bind _output_get (set `self.Instigating Character` InstigatingCharacter))
      (`/Engine/EditorBlueprintResources/StandardMacros.IsValid` `AI Interact Task`
        (:`Is Valid`
          (set `self.InteractTask` `AI Interact Task`))
        (:`Is Not Valid`
          _))
      (`/Game/Game/InteractionInterface.SetInteraction` _output_get self null)
      ; Move Player into position: trust in Player to report move completed
      (bind _asplayer_island_character_c (cast `/Game/Characters/Player/Player_IslandCharacter_C` _instigating_character)
        (:`then`
          (`/Game/Characters/Player/Player_IslandCharacter_C.PlayerAIMoveTo` _asplayer_island_character_c (`KismetMathLibrary.MakeVector` _returnvalue_x_2 _returnvalue_y_2) self))
        (:`CastFailed`
          ; Assume AI Character and move appropriately
          (bind _movementresult (`|AIMoveTo` (`Pawn.GetController` _instigating_character) _instigating_character (`KismetMathLibrary.MakeVector` _returnvalue_x_3 _returnvalue_y_3) null 100.0)
            (:`OnSuccess`
              ; Manually Reposition Actor To Interaction Spot
              (`self.K2_SetActorLocationAndRotation` _instigating_character (`KismetMathLibrary.MakeVector` _returnvalue_x _returnvalue_y _returnvalue_z) (`SceneComponent.K2_GetComponentRotation` _arrow) false false :!label _label_4)
              ; Play Entry Animations
              (`self.SetActorEnableCollision` _instigating_character false)
              (`/Engine/EditorBlueprintResources/StandardMacros.IsValid` _charactermontagein
                (:`Is Valid`
                  (`|PlayMontage` (`Character.Mesh` _instigating_character) _charactermontagein
                    (:`then`
                      (`/Engine/EditorBlueprintResources/StandardMacros.IsValid` _stationanimationin
                        (:`Is Valid`
                          (`SkeletalMeshComponent.PlayAnimation` (`self.SkeletalMesh`) _stationanimationin false))))
                    (:`OnBlendOut`
                      (goto _label))))
                (:`Is Not Valid`
                  (goto _label))))
            (:`OnFail`
              ; Report Failed move (for NPC AI) if Interaction gets blocked
              (`/Engine/EditorBlueprintResources/StandardMacros.IsValid` _interacttask
                (:`Is Valid`
                  (`/Game/Characters/NPC/AI/Tasks/Interact_Task.ReportInteractFailed` _interacttask _movementresult))))))))))

(event `self.ReportAIMoveCompleted`
  (goto _label_4))

(event `self.Continue`
  (goto _label_2))

(fn `UserConstructionScript`
  (`parent.UserConstructionScript`))