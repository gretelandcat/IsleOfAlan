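; Drivable car interactable that the island player character can enter, drive and exit, with a widget shown while highlighted.
; Interact snaps the player to a mesh socket with collision off and releases the handbrake; Continue stops the car, detaches the player to an exit point and re-engages it.
; Movement input feeds throttle, brake and steering, with cross-resetting DoOnce nodes switching driver steer-left, idle and steer-right montages only on direction changes.
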(event `self.ReceiveBeginPlay`
  (`ChaosVehicleMovementComponent.SetHandbrakeInput` (`self.VehicleMovementComponent`) true))

(event `/Game/Game/InteractionInterface.Movement`
  (params (Input :type "Vector2D Structure"))
  (bind (_x _y) (`KismetMathLibrary.BreakVector2D` Input))
  (bind _playercharacter (`self.PlayerCharacter`))
  (bind _vehiclemovementcomponent (`self.VehicleMovementComponent`))
  (`ChaosVehicleMovementComponent.SetThrottleInput` _vehiclemovementcomponent (`KismetMathLibrary.FClamp` _y))
  (`ChaosVehicleMovementComponent.SetBrakeInput` _vehiclemovementcomponent (`KismetMathLibrary.Abs` (`KismetMathLibrary.FClamp` _y -1.0 0.0)))
  (`ChaosVehicleMovementComponent.SetSteeringInput` _vehiclemovementcomponent _x)
  ; Update Driver animation based on steering (there HAS to be a better way than this!)
  (`/Engine/EditorBlueprintResources/StandardMacros.CompareFloat` _x
    (:`>`
      (`/Engine/EditorBlueprintResources/StandardMacros.DoOnce` false :!label _label
        (:`Completed`
          (`Character.PlayAnimMontage` _playercharacter "/Game/Characters/Animation/racingRight_Anim_Root_SteerRight_Montage.racingRight_Anim_Root_SteerRight_Montage" 1.0 "None")
          (`|ExecutionSequence`
            (:`then_0`
              (goto _label_2 :!via `Reset`))
            (:`then_1`
              (goto _label_3 :!via `Reset`))))))
    (:`==`
      (`/Engine/EditorBlueprintResources/StandardMacros.DoOnce` false :!label _label_2
        (:`Completed`
          (`Character.PlayAnimMontage` _playercharacter "/Game/Characters/Animation/racingIdle_Anim_Root_RacingIdle_Montage.racingIdle_Anim_Root_RacingIdle_Montage" 1.0 "None")
          (`|ExecutionSequence`
            (:`then_0`
              (goto _label :!via `Reset`))
            (:`then_1`
              (goto _label_3 :!via `Reset`))))))
    (:`<`
      (`/Engine/EditorBlueprintResources/StandardMacros.DoOnce` false :!label _label_3
        (:`Completed`
          (`Character.PlayAnimMontage` _playercharacter "/Game/Characters/Animation/racingLeft_Anim_Root_SteerLeft_Montage.racingLeft_Anim_Root_SteerLeft_Montage" 1.0 "None")
          (`|ExecutionSequence`
            (:`then_0`
              (goto _label :!via `Reset`))
            (:`then_1`
              (goto _label_2 :!via `Reset`))))))))

(event `/Game/Game/InteractionInterface.Interact`
  (params (InstigatingCharacter :type "/Game/Characters/IslandCharacter_C Object Reference") (`AI Interact Task` :type "/Game/Characters/NPC/AI/Tasks/Interact_Task Object Reference"))
  (bind _playercharacter (`self.PlayerCharacter`))
  ; Start Interaction
  (bind _output_get (set `self.PlayerCharacter` (cast `/Game/Characters/Player/Player_IslandCharacter_C` InstigatingCharacter :!pure true)))
  (`/Game/Characters/IslandCharacter_C.SetInteraction` _output_get self self)
  ; Have player drive the car!
  (`self.SetActorEnableCollision` _playercharacter false)
  (`self.K2_AttachToComponent` _playercharacter (`self.Mesh`) "PlayerAttachPoint" "SnapToTarget" "SnapToTarget" "KeepWorld" true)
  (`Character.PlayAnimMontage` _playercharacter "/Game/Characters/Animation/racingIdle_Anim_Root_RacingIdle_Montage.racingIdle_Anim_Root_RacingIdle_Montage" 1.0 "None")
  (`ChaosVehicleMovementComponent.SetHandbrakeInput` (`self.VehicleMovementComponent`) false))

(event `/Game/Game/InteractionInterface.Highlight`
  (`SceneComponent.SetVisibility` (`self.Widget`) true false))

(event `/Game/Game/InteractionInterface.DeHighlight`
  (`SceneComponent.SetVisibility` (`self.Widget`) false false))

(event `/Game/Game/InteractionInterface.Continue`
  (bind _playercharacter (`self.PlayerCharacter`))
  (`MovementComponent.StopMovementImmediately` (`self.VehicleMovementComponent`))
  (`/Game/Game/InteractionInterface.StopInteraction` (`self.PlayerCharacter`))
  (`self.K2_DetachFromActor` _playercharacter "KeepWorld" "KeepWorld" "KeepWorld")
  (`self.K2_SetActorLocation` _playercharacter (`SceneComponent.K2_GetComponentLocation` (`self.ExitPoint`)) false false)
  (`Character.StopAnimMontage` _playercharacter "/Game/Characters/Animation/racingIdle_Anim_Root_RacingIdle_Montage.racingIdle_Anim_Root_RacingIdle_Montage")
  (`self.SetActorEnableCollision` _playercharacter true)
  (`ChaosVehicleMovementComponent.SetHandbrakeInput` (`self.VehicleMovementComponent`) true))

(fn `UserConstructionScript`
  (`parent.UserConstructionScript`))